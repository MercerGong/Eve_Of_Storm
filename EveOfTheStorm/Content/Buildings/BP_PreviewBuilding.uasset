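; BP_PreviewBuilding is an actor that displays an image of a building on a plane, judging by its name as a preview.
; Its construction script looks up the building's data table row and applies a dynamic material instance to the plane.
; The Color texture comes from the row's image list at the chosen index, falling back to a random entry when that index is invalid.
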(fn `UserConstructionScript`
  (bind (_building_datatable _building_rowname) (break `DataTableRowHandle` (`self.Building`)))
  (bind _imageindex (`self.ImageIndex`))
  (bind _returnvalue (`|GetDataTableRow` _building_datatable _building_rowname)
    (:`then`
      (bind _returnvalue_2 (`KismetMaterialLibrary.CreateDynamicMaterialInstance` (`self.Material`)))
      (`PrimitiveComponent.SetMaterial` (`self.Plane`) 0 _returnvalue_2)
      (bind (_name _description _images) (break `BuildingData` _returnvalue))
      (if (`KismetArrayLibrary.Array_IsValidIndex` _images _imageindex)
        (`MaterialInstanceDynamic.SetTextureParameterValue` _returnvalue_2 "Color" (`|GetArrayItem` _images _imageindex))
        (else
          (`MaterialInstanceDynamic.SetTextureParameterValue` _returnvalue_2 "Color" (`KismetArrayLibrary.Array_Random` _images)))))))