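; Grid placement manager that snaps a BP_placeItem preview to a square grid under the mouse cursor.
; BeginPlay builds a centred array of cell positions; Tick traces under the cursor, finds the nearest cell by linear search and switches the preview material to show whether it is free.
; AddItem, not called within this Blueprint, spawns an item on a free cell and records its position, which Placeable checks by exact vector match.
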(event `self.ReceiveBeginPlay`
  (bind _returnvalue (`GameplayStatics.GetActorOfClass` "BP_GridManager_C"))
  (`self.generateGrid` _returnvalue)
  (bind _returnvalue_2 (`GameplayStatics.GetActorOfClass` "/Game/GridSystem/BP_placeItem.BP_placeItem_C"))
  (set `self.placeItem` _returnvalue_2)
  (set `PlayerController.bShowMouseCursor` true (`GameplayStatics.GetPlayerController` 0))
  (set `self.normalMat` "/Game/StarterContent/Materials/M_Brick_Clay_Beveled.M_Brick_Clay_Beveled")
  (set `self.redMat` "/Game/Material/M_transRed.M_transRed"))

(event `self.ReceiveTick`
  (params (DeltaSeconds :type "Float (single-precision)"))
  (bind (_bblockinghit _binitialoverlap _time _distance _location) (`GameplayStatics.BreakHitResult` (`PlayerController.GetHitResultUnderCursorForObjects` (`GameplayStatics.GetPlayerController` 0) (`|MakeArray` "ObjectTypeQuery7" :!type "EObjectTypeQuery Enum") true)))
  (`self.K2_SetActorLocation` (`self.placeItem`) _location false false)
  (if _bblockinghit
    (bind _returnvalue (`GameplayStatics.GetActorOfClass` "BP_GridManager_C"))
    (bind _outposiition (`self.getClosestPosition` _returnvalue _location))
    (bind _output_get (set `self.closestPosition` _outposiition))
    (`self.K2_SetActorLocation` (`self.placeItem`) (+ _output_get (0.0 0.0 10.0)) false false)
    (`GameplayStatics.GetActorOfClass` "BP_GridManager_C")
    (bind _isplaceable (`self.placeable` (`self.closestPosition`)))
    (if _isplaceable
      (bind _returnvalue_2 (`GameplayStatics.GetActorOfClass` "/Game/GridSystem/BP_placeItem.BP_placeItem_C"))
      (`PrimitiveComponent.SetMaterial` (`/Game/GridSystem/BP_placeItem.Cube` _returnvalue_2) 0 (`self.normalMat`))
      (else
        (bind _returnvalue_3 (`GameplayStatics.GetActorOfClass` "/Game/GridSystem/BP_placeItem.BP_placeItem_C"))
        (`PrimitiveComponent.SetMaterial` (`/Game/GridSystem/BP_placeItem.Cube` _returnvalue_3) 0 (`self.redMat`))))))

(event `Key|LeftMouseButton`
  (params (Key :type "Key Structure")))

(fn `addItem`
  (bind _returnvalue (`GameplayStatics.GetActorOfClass` "BP_GridManager_C"))
  (bind _isplaceable (`self.placeable` _returnvalue (`self.closestPosition`)))
  (if _isplaceable
    (bind _returnvalue_2 (`|SpawnActorFromClass` "/Game/GridSystem/BP_placeItem.BP_placeItem_C" (`KismetMathLibrary.MakeTransform` (+ (`self.closestPosition`) (0.0 0.0 10.0)) (struct) (`self.GetActorScale3D` (`self.placeItem`))) "Undefined" "OverrideRootScale" null null))
    (`PrimitiveComponent.SetMaterial` (`/Game/GridSystem/BP_placeItem.Cube` _returnvalue_2) 0 (`self.normalMat`))
    (bind _returnvalue_3 (`GameplayStatics.GetActorOfClass` "BP_GridManager_C"))
    (`self.addPositionToArray` _returnvalue_3 (`self.closestPosition`))))

(fn `addPositionToArray`
  (params (Inposition :type "Vector Structure"))
  (locals (isInclude :type Boolean))
  (bind _positionarray (`self.positionArray`))
  (set `local.isInclude` false)
  (for _array_element _positionarray
    _)
  (if (not (`local.isInclude`))
    (`KismetArrayLibrary.Array_Add` _positionarray Inposition)))

(fn `generateGrid`
  (bind _worldoffset (`self.worldoffset`))
  (bind _worldgridsize (`self.worldGridSize`))
  (bind _worldgridsize_2 (`self.worldGridSize`))
  (`KismetArrayLibrary.Array_Clear` (`self.gridArray`))
  (set `self.worldoffset` (- (* (* (`self.gridSize`) _worldgridsize) 0.5) (* _worldgridsize 0.5)))
  (for _index (range (`self.gridSize`))
    (for _index_2 (range (`self.gridSize`))
      (`KismetArrayLibrary.Array_Add` (`self.gridArray`) (+ (`KismetMathLibrary.MakeVector` (- (* _index_2 _worldgridsize_2) _worldoffset) (- (* _worldgridsize_2 _index) _worldoffset)) (0.0 0.0 10.0))))))

(fn `GeneratePosition`
  (params (InPos :type "Vector Structure"))
  (returns (gPos :type "Vector Structure"))
  (bind _outhit (`KismetSystemLibrary.LineTraceSingle` (+ InPos (0.0 0.0 1.0)) (`KismetMathLibrary.Vector_Down`) "TraceTypeQuery1"))
  (bind (_bblockinghit _binitialoverlap _time _distance _location _impactpoint) (`GameplayStatics.BreakHitResult` _outhit))
  (if _bblockinghit
    (`KismetSystemLibrary.PrintString` "Hit")
    (return (+ _impactpoint (0.0 0.0 10.0)))))

(fn `getClosestPosition`
  (params (InPosition :type "Vector Structure"))
  (returns (outPosiition :type "Vector Structure"))
  (locals (closestLocation :type "Vector Structure") (closestDistance :type "Float (double-precision)"))
  (set `local.closestLocation` InPosition)
  (set `local.closestDistance` (`KismetMathLibrary.Vector_Distance` (`|GetArrayItem` (`self.gridArray`)) InPosition))
  (for _array_element (`self.gridArray`)
    (bind _returnvalue (`KismetMathLibrary.Vector_Distance` _array_element InPosition))
    (if (< _returnvalue (`local.closestDistance`))
      (set `local.closestLocation` _array_element)
      (set `local.closestDistance` _returnvalue)))
  (return (`local.closestLocation`)))

(fn `placeable`
  (params (Inposition :type "Vector Structure"))
  (returns (isPlaceable :type Boolean))
  (locals (isp :type Boolean))
  (set `local.isp` true)
  (for _array_element (`self.positionArray`)
    (if (== Inposition _array_element)
      (set `local.isp` false)))
  (return (`local.isp`)))

(fn `UserConstructionScript`)