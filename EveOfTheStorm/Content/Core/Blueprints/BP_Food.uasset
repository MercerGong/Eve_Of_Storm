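; BP_Food is a food actor that drifts under a small physics force.
; Each tick it pushes its Sphere component with a constant upward force plus a random nudge along positive X and Y.
; A disconnected click-to-move branch, which would lerp the actor and its Plane toward TargetLocation until close, never runs, though BeginPlay still initialises its variables.
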(event `self.ReceiveBeginPlay`
  (set `self.IsClick` false)
  (set `self.moveSpeed` 5.0))

(event `self.ReceiveTick`
  (params (DeltaSeconds :type "Float (single-precision)"))
  (`PrimitiveComponent.AddForce` (`self.Sphere`) (`KismetMathLibrary.MakeVector` (* (`KismetMathLibrary.RandomFloat`) 10.0) (* (`KismetMathLibrary.RandomFloat`) 10.0) 40.0) "None" false))

(fn `UserConstructionScript`)