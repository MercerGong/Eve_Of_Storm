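; AI villager that reacts to a SearchForFood event by going to pick up a food item within its search radius.
; The event starts an AI MoveToLocation, then toggles IsPicking on the villager's Animation Blueprint and destroys the food partway through.
; Fixed delays time the sequence, with no check that the villager has arrived.
; Closest-food scan and debug sphere are unconnected, so the caller supplies the target.
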(event `self.ReceiveBeginPlay`)

(event `self.ReceiveTick`
  (params (DeltaSeconds :type "Float (single-precision)")))

(event `SearchForFood`
  (params (Location :type "Vector Structure") (food :type "Actor Object Reference"))
  (bind _searchradius (`self.SearchRadius`))
  (if (<= (`KismetMathLibrary.Vector_Distance` Location (`self.K2_GetActorLocation` self)) _searchradius)
    (`AIController.MoveToLocation` (`AIBlueprintHelperLibrary.GetAIController` self) Location (* _searchradius 0.1) false true false true null true)
    (`KismetSystemLibrary.Delay` 0.2)
    (bind _asbp_ani_villager (cast `/Game/Core/Blueprints/Villager/BP_ANI_Villager` (`SkeletalMeshComponent.GetAnimInstance` (`self.SkeletalMesh`))))
    (set `/Game/Core/Blueprints/Villager/BP_ANI_Villager.IsPicking` true _asbp_ani_villager)
    (`KismetSystemLibrary.Delay` 1.5)
    (`self.K2_DestroyActor` food)
    (`KismetSystemLibrary.Delay` 1.5)
    (set `/Game/Core/Blueprints/Villager/BP_ANI_Villager.IsPicking` false _asbp_ani_villager)))

(event `self.AnimNotify_EndJump`
  (`KismetSystemLibrary.PrintString` "endPick"))

(fn `UserConstructionScript`)