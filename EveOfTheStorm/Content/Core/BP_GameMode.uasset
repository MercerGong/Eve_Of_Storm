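; Game mode for a turn-based, tile-building resource game, won by reaching a Tech target and lost by running out of Food or turns.
; Each turn ticks BuildingSystem, deducts food consumption and checks end conditions; building events pay periodic rewards scaled by production buffs.
; Helper functions adjust price and production buffs and randomly downgrade or remove unbuilt tiles.
; Tick estimates net monthly gain and, in later turns, drives a thunderstorm with dimming light.
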(event `self.ReceiveBeginPlay`
  (`GameplayStatics.PlaySound2D` "/Game/Audio/Ambient/SW_Month_Remind.SW_Month_Remind" 1.0 1.0 0.0 null null)
  (add `ESBuildingSystem.OnBuildingTriggerEvent` (`self.BuildingSystem`) (delegate `OnBuilding Event`))
  (add `self.GameTurnEvent` (delegate `GameTurnEvent_Event`))
  (bind _asbp_player_state (cast `/Game/Core/BP_PlayerState` (`Controller.PlayerState` (`GameplayStatics.GetPlayerController` 0))))
  (bind _output_get (set `self.PS` _asbp_player_state))
  (set `self.LastMonthAdded` (* (`ESPlayerState.CurrentConsumeFood` _output_get) -1.0))
  (set `self.StartWeatherChange` false)
  (set `self.TransitionTime` 10.0))

(event `GameTurnEvent_Event` :!signature `self.GameTurnEvent`
  (params (CurrentTurn :type Integer))
  (bind _returnvalue (`GameplayStatics.GetPlayerController` 0))
  (bind _resourcesystem (`ESPlayerState.ResourceSystem` (`self.PS`)))
  (if (>= CurrentTurn 19)
    (bind _asbp_player_controller (cast `/Game/Core/BP_PlayerController` (`GameplayStatics.GetPlayerController` 0)))
    (`/Game/Core/BP_PlayerController.OnEnd` _asbp_player_controller false)
    (`GameplayStatics.SetGamePaused` true)
    (else
      (set `self.StartWeatherChange` (>= CurrentTurn 12))
      (`GameplayStatics.PlaySound2D` "/Game/Audio/Ambient/SW_Month_Remind.SW_Month_Remind" 1.0 1.0 0.0 null null)
      (set `self.LastMonthAdded` 0.0)
      (bind _buff (`self.GetProductionBuff`))
      (set `self.CurrentBuff` _buff)
      (`ESBuildingSystem.TickBuilding` (`self.BuildingSystem`))
      (bind _asbp_player_state (cast `/Game/Core/BP_PlayerState` (`Controller.PlayerState` (`GameplayStatics.GetPlayerController` 0))))
      (bind _currentconsumefood (`ESPlayerState.CurrentConsumeFood` _asbp_player_state))
      (set `self.LastMonthAdded` (- (`self.LastMonthAdded`) _currentconsumefood))
      (`ESGameHelper.ApplyResourceModifier` (`GameplayStatics.GetPlayerController` 0) (make `ResourceModifier` "Food" "Additive" (* _currentconsumefood -1.0)))
      (`ESPlayerState.OnTurn` _asbp_player_state)
      (set `self.TurnCount` (+ (`self.TurnCount`) 1))
      (`ESResourceSystem.SetMaxResourceValue` _resourcesystem "Tech" (`ESResourceSystem.GetResourceValue` _resourcesystem "MaxTech"))
      (bind _returnvalue_2 (`ESGameHelper.GetResource` _returnvalue "Food"))
      (if (== _returnvalue_2 0.0)
        (`KismetSystemLibrary.PrintString` "You Lose")
        (bind _asbp_player_controller_2 (cast `/Game/Core/BP_PlayerController` (`GameplayStatics.GetPlayerController` 0)))
        (`/Game/Core/BP_PlayerController.OnEnd` _asbp_player_controller_2 false)
        (`GameplayStatics.SetGamePaused` true)
        (else
          (bind _returnvalue_3 (`ESGameHelper.GetResource` _returnvalue "Tech"))
          (if (>= _returnvalue_3 1000.0)
            (`KismetSystemLibrary.PrintString` "You Win")
            (bind _asbp_player_controller_3 (cast `/Game/Core/BP_PlayerController` (`GameplayStatics.GetPlayerController` 0)))
            (`/Game/Core/BP_PlayerController.OnEnd` _asbp_player_controller_3 true)
            (`GameplayStatics.SetGamePaused` true)))))))

(event `OnBuilding Event`
  (params (BuildinData :type "BuildingData Structure (by ref)") (EventCount :type Integer))
  (for _array_element (`.Rewards` (break `BuildingData` BuildinData))
    (bind (_period _resourcetype _resourceamount) (break `BuildRewardPeriod` _array_element))
    (if (== (mod EventCount _period) 0)
      (bind _returnvalue (* _resourceamount (`self.CurrentBuff`)))
      (`ESGameHelper.ApplyResourceModifier` (`GameplayStatics.GetPlayerController` 0) (make `ResourceModifier` _resourcetype "Additive" _returnvalue))
      (set `self.LastMonthAdded` (+ _returnvalue (`self.LastMonthAdded`))))))

(event `self.ReceiveTick`
  (params (DeltaSeconds :type "Float (single-precision)"))
  (bind _returnvalue (`ESBuildingSystem.GetEstimateCost` (`self.BuildingSystem`)))
  (bind _buff (`self.GetProductionBuff`))
  (set `self.LastMonthAdded` (- (* _returnvalue _buff) (`ESPlayerState.CurrentConsumeFood` (`self.PS`))))
  (if (`self.StartWeatherChange`)
    (`self.StartThunderStorm` (`self.TransitionTime`) DeltaSeconds)))

(fn `DowngradeLand`
  (params (Count :type Integer))
  (locals (LoopCount :type Integer) (RandomIndex :type Integer :default 0) (RandomPoint :type "IntPoint Structure") (Points :type "Array of IntPoint Structure") (`Removing Points` :type "Array of IntPoint Structure"))
  (bind _points (`local.Points`))
  (`GameplayStatics.PlaySound2D` "/Game/Audio/Feedback/Debuff_Downgrade_Cue.Debuff_Downgrade_Cue" 1.0 1.0 0.0 null null)
  (set `local.LoopCount` Count)
  (bind _returnvalue (`ESGridSystem.GetPoints` (`self.GridSystem`) 0))
  (bind _output_get (set `local.Points` _returnvalue))
  (while (and (`KismetArrayLibrary.Array_IsNotEmpty` _output_get) (> (`local.LoopCount`) 0))
    (bind _output_get_2 (set `local.RandomIndex` (`.OutIndex` (`KismetArrayLibrary.Array_Random` _output_get))))
    (bind _output_get_3 (set `local.RandomPoint` (`|GetArrayItem` _points _output_get_2)))
    (`KismetArrayLibrary.Array_Remove` _points _output_get_2)
    (bind (_x _y) (break `IntPoint` _output_get_3))
    (if (and (not (`ESBuildingSystem.HasBuilding` (`self.BuildingSystem`) _output_get_3)) (> (`ESGridSystem.GetTileType` (`self.GridSystem`) _x _y) 1))
      (`KismetArrayLibrary.Array_Add` (`local.Removing Points`) (`local.RandomPoint`))
      (`/Engine/EditorBlueprintResources/StandardMacros.DecrementInt` (`local.LoopCount`))))
  (for _array_element (`local.Removing Points`)
    (bind (_x_2 _y_2) (break `IntPoint` _array_element))
    (bind _returnvalue_2 (`ESGridSystem.GetTileType` (`self.GridSystem`) _x_2 _y_2))
    (if (`|EnumEquality` _returnvalue_2 "Sand")
      (bind (_x_3 _y_3) (break `IntPoint` _array_element))
      (`ESGridSystem.UpdateOneTile` (`self.GridSystem`) _x_3 _y_3 (cast `EGroundType` (- _returnvalue_2 1)))))
  (for _array_element_2 (`local.Removing Points`)
    (bind (_x_4 _y_4) (break `IntPoint` _array_element_2))
    (bind _returnvalue_3 (`ESGridSystem.GetTileType` (`self.GridSystem`) _x_4 _y_4))
    (if (`|EnumEquality` _returnvalue_3 "Grass")
      (bind (_x_5 _y_5) (break `IntPoint` _array_element_2))
      (`ESGridSystem.UpdateOneTile` (`self.GridSystem`) _x_5 _y_5 (cast `EGroundType` (- _returnvalue_3 1))))))

(fn `GetProductionBuff`
  (returns (Buff :type "Float (double-precision)"))
  (locals (Result :type "Float (double-precision)"))
  (for _array_element (`self.ProductionBuffList`)
    (set `local.Result` (+ (`local.Result`) (/ (`.Precentage_2_A2D59EB94917218449A65AA024CD1E9C` (break `/Game/Core/Blueprints/ProductionType` _array_element)) 100.0))))
  (return (+ (`local.Result`) 1.0)))

(fn `RemoveRandomLand`
  (params (Count :type Integer))
  (locals (i :type Integer) (Points :type "Array of IntPoint Structure") (RandomI :type Integer :default 0) (CachePoint :type "IntPoint Structure"))
  (bind (_cachepoint_x _cachepoint_y) (break `IntPoint` (`local.CachePoint`)))
  (bind _points (`local.Points`))
  (bind _output_get (set `local.i` Count))
  (bind _returnvalue (`ESGridSystem.GetPoints` (`self.GridSystem`) 0))
  (bind _output_get_2 (set `local.Points` _returnvalue))
  (while (or (> _output_get 0) (`KismetArrayLibrary.Array_IsEmpty` _output_get_2))
    (bind _output_get_3 (set `local.RandomI` (`.OutIndex` (`KismetArrayLibrary.Array_Random` _points))))
    (bind _output_get_4 (set `local.CachePoint` (`|GetArrayItem` _points _output_get_3)))
    (`KismetArrayLibrary.Array_Remove` (`local.Points`) _output_get_3)
    (if (not (`ESBuildingSystem.HasBuilding` (`self.BuildingSystem`) _output_get_4))
      (`/Engine/EditorBlueprintResources/StandardMacros.DecrementInt` (`local.i`)
        (:`  `
          (`ESGridSystem.RemoveOneTile` (`self.GridSystem`) _cachepoint_x _cachepoint_y))))))

(fn `StartThunderStorm`
  (params (`TransitionTime(Sec)` :type "Float (double-precision)") (deltaTime :type "Float (double-precision)"))
  (locals (LightIntensity :type "Float (double-precision)"))
  (bind _returnvalue (`GameplayStatics.GetActorOfClass` "/Game/UltraDynamicSky/Blueprints/Ultra_Dynamic_Weather.Ultra_Dynamic_Weather_C"))
  (`/Game/UltraDynamicSky/Blueprints/Ultra_Dynamic_Weather.Change Weather` _returnvalue "/Game/UltraDynamicSky/Blueprints/Weather_Effects/Weather_Presets/Rain_Thunderstorm.Rain_Thunderstorm" `TransitionTime(Sec)` false)
  (if (`self.StartWeatherChange`)
    (bind _returnvalue_2 (`GameplayStatics.GetActorOfClass` "/Script/Engine.DirectionalLight"))
    (bind _lightcomponent (`Light.LightComponent` _returnvalue_2))
    (set `local.LightIntensity` (`LightComponentBase.Intensity` _lightcomponent))
    (if (>= (`local.LightIntensity`) 3.8)
      (`LightComponent.SetIntensity` _lightcomponent (- (`local.LightIntensity`) (* deltaTime 2.5)))
      (else
        (set `self.StartWeatherChange` false)))))

(fn `TurnProduction Buff`
  (bind _productionbufflist (`self.ProductionBuffList`))
  (bind (_arrayindex _arrayelement) (`/Engine/EditorBlueprintResources/StandardMacros.ReverseForEachLoop` _productionbufflist)
    (:`LoopBody`
      (bind (_precentage _month) (break `/Game/Core/Blueprints/ProductionType` _arrayelement))
      (bind _result (`/Engine/EditorBlueprintResources/StandardMacros.DecrementInt` _month)
        (:`  `
          (if (< _result _month)
            (`KismetArrayLibrary.Array_Remove` _productionbufflist _arrayindex)))))))

(fn `UpdateFoodProduction`
  (params (Precent :type "Float (double-precision)") (Month :type Integer))
  (locals (Count :type Integer))
  (`KismetArrayLibrary.Array_Add` (`self.ProductionBuffList`) (make `/Game/Core/Blueprints/ProductionType` Precent Month)))

(fn `UpdatePriceBuff`
  (params (Precent :type "Float (double-precision)"))
  (bind _asbp_player_state (cast `/Game/Core/BP_PlayerState` (`Controller.PlayerState` (`GameplayStatics.GetPlayerController` 0))))
  (set `ESPlayerState.CurrentDrawBuff` (+ (`ESPlayerState.CurrentDrawBuff` _asbp_player_state) (/ Precent 100.0)) _asbp_player_state))

(fn `UpdatePriceBuffTempo`
  (params (Precent :type "Float (double-precision)"))
  (bind _asbp_player_state (cast `/Game/Core/BP_PlayerState` (`Controller.PlayerState` (`GameplayStatics.GetPlayerController` 0))))
  (set `ESPlayerState.CurrentDrawBuffTempo` (+ (`ESPlayerState.CurrentDrawBuffTempo` _asbp_player_state) (/ Precent 100.0)) _asbp_player_state))

(fn `UserConstructionScript`)