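; Player pawn that plays an intro camera zoom on start and then smooths later changes to its zoom distance.
; After a short delay, the ZoomOut timeline drives both the camera boom length and TargetZoom.
; When it finishes, the pawn sets its movement speed and enables interpolation on Tick, easing the boom toward TargetZoom.
; No zoom input appears in these graphs.
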(event `self.ReceiveBeginPlay`
  (bind _defaultzoom (`self.DefaultZoom`))
  (set `SpringArmComponent.TargetArmLength` _defaultzoom (`self.CameraBoom`))
  (set `self.TargetZoom` _defaultzoom)
  (`KismetSystemLibrary.Delay` 0.5)
  (bind (_direction _camera) (`Timeline|ZoomOut`)
    (:`Update`
      (set `SpringArmComponent.TargetArmLength` _camera (`self.CameraBoom`))
      (set `self.TargetZoom` _camera))
    (:`Finished`
      (set `FloatingPawnMovement.MaxSpeed` 2500.0 (`self.PawnMovement`))
      (set `self.StartZoom` true))))

(event `self.ReceiveTick`
  (params (DeltaSeconds :type "Float (single-precision)"))
  (bind _targetzoom (`self.TargetZoom`))
  (bind _targetarmlength (`SpringArmComponent.TargetArmLength` (`self.CameraBoom`)))
  (if (`self.StartZoom`)
    (if (!= _targetzoom _targetarmlength)
      (set `SpringArmComponent.TargetArmLength` (`KismetMathLibrary.FInterpTo` _targetarmlength _targetzoom DeltaSeconds 10.0) (`self.CameraBoom`)))))

(fn `UserConstructionScript`)