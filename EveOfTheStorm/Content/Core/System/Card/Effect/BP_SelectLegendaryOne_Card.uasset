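; BP_SelectLegendaryOne_Card is a card effect that offers the player a choice from three random Legendary cards.
; OnEffect casts to BP_PlayerController, gets the card manager from its GameUI, draws three random Legendary cards and passes them to OnCardSelect.
; CanApplyEffect always returns true; a card manager CanDraw check exists in the graph but never runs.
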(event `self.K2_OnEffect`
  (params (GameMode :type "ESDefaultGameMode Object Reference") (PlayerController :type "PlayerController Object Reference"))
  (bind _asbp_player_controller (cast `/Game/Core/BP_PlayerController` PlayerController))
  (bind _cardsystem (`/Game/Core/UI/WBP_GameUI.GetCardManager` (`/Game/Core/BP_PlayerController.GameUI` _asbp_player_controller)))
  (bind _3cardlist1 (`/Game/Core/UI/WBP_CardManager.DrawRandomThreeCard` _cardsystem "Legendary"))
  (`/Game/Core/BP_PlayerController.OnCardSelect` _asbp_player_controller _3cardlist1))

(fn `K2_CanApplyEffect`
  (params (GameMode :type "ESDefaultGameMode Object Reference") (PlayerController :type "PlayerController Object Reference"))
  (returns (CanApply :type Boolean))
  (return true))