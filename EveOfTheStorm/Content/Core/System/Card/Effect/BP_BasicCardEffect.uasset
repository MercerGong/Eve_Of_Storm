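; BP_BasicCardEffect is a skeleton card effect for the card system, with no gameplay result of its own.
; OnEffect casts to the project's game mode, player controller and player state and fetches the card manager from the game UI, then ends.
; K2_CanApplyEffect always allows the effect.
; Food resource lookup, card removal and grid and building system references are present but unconnected or unused.
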(event `self.K2_OnEffect`
  (params (GameMode :type "ESDefaultGameMode Object Reference") (PlayerController :type "PlayerController Object Reference"))
  (bind _asbp_game_mode (cast `/Game/Core/BP_GameMode` GameMode))
  (bind _asbp_player_controller (cast `/Game/Core/BP_PlayerController` PlayerController))
  (bind _cardsystem (`/Game/Core/UI/WBP_GameUI.GetCardManager` (`/Game/Core/BP_PlayerController.GameUI` _asbp_player_controller)))
  (cast `/Game/Core/BP_PlayerState` (`Controller.PlayerState` _asbp_player_controller)))

(fn `K2_CanApplyEffect`
  (params (GameMode :type "ESDefaultGameMode Object Reference") (PlayerController :type "PlayerController Object Reference"))
  (returns (CanApply :type Boolean))
  (return true))