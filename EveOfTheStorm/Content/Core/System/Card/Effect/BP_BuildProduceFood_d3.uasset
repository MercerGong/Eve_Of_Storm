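; Card effect that grants Legendary-rarity cards based on how many buildings fail the CanProduceFood check, despite the asset's BuildProduceFood name.
; OnEffect counts those entries in the BuildingSystem's BuildingData, then adds one card per full five through the GameUI's card manager.
; K2CanApplyEffect repeats the count and allows the effect only at five or more.
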(event `self.K2_OnEffect`
  (params (GameMode :type "ESDefaultGameMode Object Reference") (PlayerController :type "PlayerController Object Reference"))
  (bind _canproducenum (`self.canProduceNum`))
  (set `self.Mutiply` 0)
  (set `self.canProduceNum` 0)
  (bind _asbp_game_mode (cast `/Game/Core/BP_GameMode` GameMode))
  (bind _asbp_player_controller (cast `/Game/Core/BP_PlayerController` PlayerController))
  (for _array_element (`ESBuildingSystem.BuildingData` (`ESDefaultGameMode.BuildingSystem` _asbp_game_mode))
    (if (not (`ESGridHelper.CanProduceFood` (`.Data` (break `BuildingInfo` _array_element))))
      (set `self.canProduceNum` (+ (`self.canProduceNum`) 1))))
  (if (>= (`self.canProduceNum`) 5)
    (while (> (`self.canProduceNum`) 0)
      (set `self.canProduceNum` (- _canproducenum (mod _canproducenum 5)))
      (set `self.canProduceNum` (- (`self.canProduceNum`) 5))
      (set `self.Mutiply` (+ (`self.Mutiply`) 1)))
    (for _ (range (`self.Mutiply`))
      (bind _cardsystem (`/Game/Core/UI/WBP_GameUI.GetCardManager` (`/Game/Core/BP_PlayerController.GameUI` _asbp_player_controller)))
      (`/Game/Core/UI/WBP_CardManager.AddCard_BaseOnRaity` _cardsystem "Legendary"))))

(fn `K2_CanApplyEffect`
  (params (GameMode :type "ESDefaultGameMode Object Reference") (PlayerController :type "PlayerController Object Reference"))
  (returns (CanApply :type Boolean))
  (set `self.canProduceNum` 0)
  (bind _asbp_game_mode (cast `/Game/Core/BP_GameMode` GameMode))
  (bind _asbp_player_controller (cast `/Game/Core/BP_PlayerController` PlayerController))
  (for _array_element (`ESBuildingSystem.BuildingData` (`ESDefaultGameMode.BuildingSystem` _asbp_game_mode))
    (if (not (`ESGridHelper.CanProduceFood` (`.Data` (break `BuildingInfo` _array_element))))
      (set `self.canProduceNum` (+ (`self.canProduceNum`) 1))))
  (if (>= (`self.canProduceNum`) 5)
    (return true)
    (else
      (return false))))