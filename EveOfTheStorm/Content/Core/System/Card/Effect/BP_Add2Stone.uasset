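; BP_Add2Stone is a card effect that gives the player two Stone cards.
; On effect, it looks up the Stone row in the DT_HiddenCard data table and has the card manager from the player's game UI draw that specific card twice.
; The effect can apply only when the player controller's card manager reports it can draw two cards.
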(event `self.K2_OnEffect`
  (params (GameMode :type "ESDefaultGameMode Object Reference") (PlayerController :type "PlayerController Object Reference"))
  (bind _asbp_player_controller (cast `/Game/Core/BP_PlayerController` PlayerController))
  (bind _cardsystem (`/Game/Core/UI/WBP_GameUI.GetCardManager` (`/Game/Core/BP_PlayerController.GameUI` _asbp_player_controller)))
  (bind _returnvalue (`|GetDataTableRow` "/Game/Core/Card/Basic/DT_HiddenCard.DT_HiddenCard" "Stone")
    (:`then`
      (for _index (range 2)
        (`/Game/Core/UI/WBP_CardManager.DrawSpecifyCard` _cardsystem _returnvalue)))))

(fn `K2_CanApplyEffect`
  (params (GameMode :type "ESDefaultGameMode Object Reference") (PlayerController :type "PlayerController Object Reference"))
  (returns (CanApply :type Boolean))
  (bind _asbp_player_controller (cast `/Game/Core/BP_PlayerController` PlayerController)
    (:`then`
      (return (`/Game/Core/UI/WBP_CardManager.CanDraw` (`/Game/Core/BP_PlayerController.Card Manager` _asbp_player_controller) 2)))
    (:`CastFailed`
      (return false))))