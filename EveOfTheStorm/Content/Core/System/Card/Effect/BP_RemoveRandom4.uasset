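; Card effect that removes random cards from the player's cards, applicable only when more than three are present.
; On effect, it gets the card manager through the player controller's game UI and calls its random removal in a loop over indices 0 to 2, despite the "4" in the asset name.
; The applicability check reads the card count from the same manager.
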(event `self.K2_OnEffect`
  (params (GameMode :type "ESDefaultGameMode Object Reference") (PlayerController :type "PlayerController Object Reference"))
  (bind _asbp_player_controller (cast `/Game/Core/BP_PlayerController` PlayerController))
  (bind _cardsystem (`/Game/Core/UI/WBP_GameUI.GetCardManager` (`/Game/Core/BP_PlayerController.GameUI` _asbp_player_controller)))
  (for _index (range 3)
    (`/Game/Core/UI/WBP_CardManager.Remove_Random` _cardsystem)))

(fn `K2_CanApplyEffect`
  (params (GameMode :type "ESDefaultGameMode Object Reference") (PlayerController :type "PlayerController Object Reference"))
  (returns (CanApply :type Boolean))
  (bind _asbp_player_controller (cast `/Game/Core/BP_PlayerController` PlayerController))
  (bind _cardsystem (`/Game/Core/UI/WBP_GameUI.GetCardManager` (`/Game/Core/BP_PlayerController.GameUI` _asbp_player_controller)))
  (bind _returnvalue (`/Game/Core/UI/WBP_CardManager.Get_Card_Num` _cardsystem))
  (return (> _returnvalue 3)))