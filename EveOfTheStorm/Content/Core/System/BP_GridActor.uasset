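; BP_GridActor is the grid actor that adds visual and audio feedback when tiles spawn or are destroyed.
; On spawn, it looks up the ground type's mesh in GridMeshes and spawns a BP_BlockSpawnAnimator for that instance index.
; On destruction, it spawns a BP_BlockDestroyAnimator at the tile's transform with that type's GroundMaterials and plays a 2D destroy sound.
; Either effect is skipped when the ground type has no map entry.
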(event `self.OnTileSpawned`
  (params (GroundType :type "EGroundType Enum" :default "None") (Index :type Integer))
  (bind (_value _returnvalue) (`BlueprintMapLibrary.Map_Find` (`self.GridMeshes`) GroundType))
  (if _returnvalue
    (`|SpawnActorFromClass` "/Game/Core/System/Animation/BP_BlockSpawnAnimator.BP_BlockSpawnAnimator_C" (`KismetMathLibrary.MakeTransform` (0.0 0.0 0.0)) "Undefined" "MultiplyWithRoot" null _value Index false null)))

(event `self.OnTileDestroyed`
  (params (GroundType :type "EGroundType Enum" :default "None") (X :type Integer) (Y :type Integer))
  (bind (_value _returnvalue) (`BlueprintMapLibrary.Map_Find` (`self.GroundMaterials`) GroundType))
  (bind _returnvalue_2 (`self.GetTileTransform` X Y))
  (if _returnvalue
    (`|SpawnActorFromClass` "/Game/Core/System/Animation/BP_BlockDestroyAnimator.BP_BlockDestroyAnimator_C" _returnvalue_2 "Undefined" "MultiplyWithRoot" null (`.Materials` (break `BlockMaterial` _value)) null)
    (`GameplayStatics.PlaySound2D` "/Game/Audio/Feedback/Destroy_Blocks_Cue.Destroy_Blocks_Cue" 1.0 1.0 0.0 null null)))

(fn `UserConstructionScript`)