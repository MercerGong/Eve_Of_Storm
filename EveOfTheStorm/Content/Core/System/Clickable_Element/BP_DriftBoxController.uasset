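; AI controller that sends its drift box pawn wandering, then removes it after a limited lifetime.
; On BeginPlay it sets a fixed target area and starts a looping timer, with a negative start delay cancelling the first wait.
; Each Drift call moves the pawn to a random reachable navigation point around that area.
; Tick destroys the pawn once the controller has existed for over a minute.
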(event `self.ReceiveBeginPlay`
  (set `self.movetoPosition` (-5000.0 -5000.0 -110.0))
  (`KismetSystemLibrary.K2_SetTimerDelegate` (delegate `Drift`) 60.0 true -60.0))

(event `Drift`
  (`|AIMoveTo` (`self.K2_GetPawn`) (`NavigationSystemV1.K2_GetRandomReachablePointInRadius` (`self.movetoPosition`) 2000.0 null null) null 360.0 true))

(event `self.ReceiveTick`
  (params (DeltaSeconds :type "Float (single-precision)"))
  (if (> (`self.GetGameTimeSinceCreation`) 60.0)
    (`self.K2_DestroyActor` (`self.K2_GetPawn`))))

(fn `UserConstructionScript`)